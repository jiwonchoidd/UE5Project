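; Player character Blueprint with two switchable cameras and a decal that marks the surface under the mouse cursor.
; BeginPlay switches to Camera2 if Camera1 is active, and the C key toggles between the two through the CurrentCamera variable.
; Every Tick, a complex Visibility trace under the cursor moves the decal to the hit location and aligns it to the impact normal.
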(event EventBeginPlay
  (bind _camera2 (Variables|Default|GetCamera2))
  ;[1 1 1] 기본카메라 세팅
  (if (Components|Activation|IsActive (Variables|Default|GetCamera1))
    (Components|Activation|Deactivate (Variables|Default|GetCamera1))
    (Components|Activation|Activate _camera2 false)
    (Variables|Default|SetCurrentCamera _camera2)))

(event EventTick
  (params (DeltaSeconds :type Float%20%28single-precision%29))
  (bind _returnvalue (Game|GetPlayerController 0))
  (bind _hitresult (Game|Player|GetHitResultUnderCursorbyChannel _returnvalue "TraceTypeQuery1" true))
  (bind (_bblockinghit _binitialoverlap _time _distance _location _impactpoint _normal _impactnormal) (Collision|BreakHitResult _hitresult))
  ;[1 1 1] 코멘트
  (Transformation|SetWorldLocationAndRotation (Variables|Default|GetDecal) _location (Math|Rotator|MakeRotationfromAxes _impactnormal "0, 0, 0" "0, 0, 0") false false))

(event Input|KeyboardEvents|C
  (params (Key :type Key%20Structure :default "None"))
  (bind _camera2 (Variables|Default|GetCamera2))
  (bind _camera1 (Variables|Default|GetCamera1))
  ;[1 1 1] 케메라전환
  (:Pressed
    (Components|Activation|Deactivate (Variables|Default|GetCurrentCamera))
    (if (== (Variables|Default|GetCurrentCamera) (Variables|Default|GetCamera1))
      (Components|Activation|Activate _camera2 false)
      (Variables|Default|SetCurrentCamera _camera2)
      (else
        (Components|Activation|Activate _camera1 false)
        (Variables|Default|SetCurrentCamera _camera1)))))

(fn ConstructionScript)