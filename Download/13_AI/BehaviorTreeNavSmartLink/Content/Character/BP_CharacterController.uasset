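; BP_CharacterController is a player controller that provides click-to-move for its pawn.
; Holding the SetDestination input opens a gate, so every Tick traces the hit under the cursor on the Visibility channel and passes it to MoveToHitLocation.
; That function calls SimpleMoveToLocation only when the hit is at least a short threshold distance from the pawn, skipping moves to points right beside it.
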(event EventBeginPlay)

(event EventTick
  (params (DeltaSeconds :type Float%20%28single-precision%29))
  (Utilities|FlowControl|Gate true
    (:Exit
      (CallFunction|MovetoHitLocation (.HitResult (Game|Player|GetHitResultUnderCursorbyChannel "TraceTypeQuery1" true))))))

(event Input|ActionEvents|InputActionSetDestination
  (params (Key :type Key%20Structure))
  (:Pressed
    (Utilities|FlowControl|Gate true) ; enters at Open
  )
  (:Released
    (Utilities|FlowControl|Gate true) ; enters at Close
  ))

(fn ConstructionScript)

(fn MovetoHitLocation
  (params (hit :type Hit%20Result%20Structure))
  (bind _location (Collision|BreakHitResult hit))
  (if (>= (Math|Vector|VectorLength (- (Transformation|GetActorLocation (Pawn|GetControlledPawn)) _location)) 1.2e+02)
    (AI|Navigation|SimpleMovetoLocation self _location)))