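; GM_AI is an AI game mode Blueprint that spawns enemies around the player during play.
; A looping timer started on BeginPlay picks a random navigable point within a radius of the player pawn and randomly spawns one of two child enemy classes there.
; Each spawn increments and prints a counter, and the timer is cleared once the counter reaches the maximum.
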(event Custom|SpawnEnemy
  ;[1 1 1] Enemy Spawn
  (if (> (Variables|Default|GetMaxEnemyCounter) (Variables|Default|GetEnemyCounter))
    (bind (_randomlocation _returnvalue) (Class|NavigationSystemV1|GetRandomLocationinNavigableRadius (Transformation|GetActorLocation (Game|Player|GetPlayerPawn 0)) 3e+03 0 0))
    (if _returnvalue
      (if (Math|Random|RandomBool)
        (Game|SpawnActorfromClass "/Game/ai/BP_ChildEnemy1.BP_ChildEnemy1_C" (Math|Transform|MakeTransform _randomlocation) "Undefined" 0 0)
        (else
          (Game|SpawnActorfromClass "/Game/ai/BP_ChildEnemy2.BP_ChildEnemy2_C" (Math|Transform|MakeTransform _randomlocation) "Undefined" 0 0)))
      (bind _output_get (Variables|Default|SetEnemyCounter (+ (Variables|Default|GetEnemyCounter) 1)))
      (Development|PrintString (Utilities|String|ToString(Integer) _output_get)))
    (else
      (Utilities|Time|ClearandInvalidateTimerbyHandle (Variables|Default|GetSpawnTimter)))))

(event EventBeginPlay
  ;[1 1 1] Enemy Spawn
  (bind _returnvalue (Utilities|Time|SetTimerbyEvent (delegate Custom|SpawnEnemy) (Variables|Default|GetSpawnTime) true))
  (Variables|Default|SetSpawnTimter _returnvalue))

(fn ConstructionScript)