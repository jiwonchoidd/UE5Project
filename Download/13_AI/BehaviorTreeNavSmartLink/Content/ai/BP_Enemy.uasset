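; BP_Enemy is an AI enemy character that tracks the player through AI Perception and reports it to its Blackboard.
; Sensing an actor tagged Player cancels the forget timer, sets the line-of-sight flag and stores that actor.
; Any other perception update starts a short timer that clears both Blackboard entries when it expires.
; An UpdateWalkSpeed event lets callers change the movement speed.
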(event OnTargetPerceptionUpdated(AIPerception)
  (params (Actor :type Actor%20Object%20Reference) (Stimulus :type AI%20Stimulus%20Structure))
  (bind _returnvalue (AI|GetBlackboard 0))
  ;[1 1 1] 코멘트
  (if (and (Actor|ActorHasTag Actor "Player") (.bSuccessfullySensed (Utilities|Struct|BreakAIStimulus Stimulus)))
    (Utilities|Time|ClearandInvalidateTimerbyHandle (Variables|Default|GetEnemyTimer))
    (AI|Components|Blackboard|SetValueasBool _returnvalue (Variables|Default|GetHasLineOfSight) true)
    (AI|Components|Blackboard|SetValueasObject _returnvalue (Variables|Default|GetKey%20Name) Actor)
    (else
      (bind _returnvalue_2 (Utilities|Time|SetTimerbyEvent (delegate Custom|커스텀이벤트_0) 3.0))
      (Variables|Default|SetEnemyTimer _returnvalue_2))))

(event Custom|UpdateWalkSpeed
  (params (Newspeed :type Float%20%28single-precision%29))
  ;[1 1 1] 코멘트
  (Variables|/Script/Engine.CharacterMovementComponent|SetMaxWalkSpeed (Variables|Character|GetCharacterMovement) Newspeed))

(event Custom|커스텀이벤트_0
  (bind _returnvalue (AI|GetBlackboard 0))
  ;[1 1 1] 코멘트
  (AI|Components|Blackboard|SetValueasBool _returnvalue (Variables|Default|GetHasLineOfSight) false)
  (AI|Components|Blackboard|SetValueasObject _returnvalue (Variables|Default|GetKey%20Name) 0))

(fn ConstructionScript)