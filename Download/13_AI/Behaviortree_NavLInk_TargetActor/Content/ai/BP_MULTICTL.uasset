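; AI controller that runs a follower behavior tree, saving the pawn's spawn position as HomeLocation in its blackboard.
; It also defines movement helpers, not called in this graph: MoveTypeA wanders to a random nearby point.
; MoveTypeB moves forward without pathfinding, stepping right when a visibility trace ahead hits something.
; GetRandomTargetLocation shuffles all WayPoint actors and returns the first one's location.
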(event EventBeginPlay
  ;[1 1 1] 코멘트
  (Class|AIController|UseBlackboard "/Game/ai/FollowerBlackboard.FollowerBlackboard")
  (AI|Components|Blackboard|SetValueasVector (AI|GetBlackboard 0) (Variables|KGCA|GetHomeLocation) (Transformation|GetActorLocation (Pawn|GetControlledPawn)))
  (AI|RunBehaviorTree "/Game/ai/FollowerBT.FollowerBT"))

(fn ConstructionScript)

(fn MoveTypeA
  ;[1 1 1] 코멘트
  (AI|Navigation|MovetoLocation (+ (Math|Vector|MakeVector (Math|Random|RandomFloatinRange -555.0 555.0) (Math|Random|RandomFloatinRange -555.0 555.0) 0.0) (Transformation|GetActorLocation (Pawn|GetControlledPawn))) -1.0 true true false true 0))

(fn MoveTypeB
  (bind _returnvalue (Pawn|GetControlledPawn))
  (bind _returnvalue_2 (Transformation|GetActorLocation _returnvalue))
  (bind _returnvalue_3 (Transformation|GetActorForwardVector _returnvalue))
  (bind _returnvalue_4 (* _returnvalue_3 255.0))
  (bind _returnvalue_5 (+ _returnvalue_2 _returnvalue_4))
  ;[1 1 1] 코멘트
  (bind _returnvalue_6 (Collision|LineTraceByChannel _returnvalue_2 _returnvalue_5 "TraceTypeQuery1" false 0 "None"))
  (AI|Navigation|MovetoLocation (Math|Vector|SelectVector (+ (* (Transformation|GetActorRightVector _returnvalue) 255.0) (Transformation|GetActorLocation _returnvalue)) _returnvalue_5 _returnvalue_6) -1.0 true false false true 0))

(fn GetRandomTargetLocation
  ;[1 1 1] 랜덤하게 타켓 엑터의 위치를 반환한다.
  (bind _outactors (Actor|GetAllActorsOfClass "/Game/ai/WayPoint.WayPoint_C"))
  (bind _output_get (Variables|Default|SetTargetArray _outactors))
  (Utilities|Array|Shuffle _output_get)
  (bind _output_get_2 (Variables|Default|SetTarget (Utilities|Array|Get(acopy) _output_get)))
  (return (Transformation|GetActorLocation _output_get_2)))