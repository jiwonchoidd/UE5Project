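; GM_AI, apparently a game mode, spawns enemies around the player up to a set maximum.
; A looping timer started on BeginPlay picks a random navigable point within a fixed radius of the player pawn each tick.
; When a point is found, it spawns one of three random child enemy classes there and increments the counter.
; Once the counter reaches the maximum, the timer is cleared, and nothing here restarts it.
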(event Custom|SpawnEnemy
  (if (> (Variables|Default|GetMaxEnemyCounter) (Variables|Default|GetEnemyCounter))
    (bind (_randomlocation _returnvalue) (Class|NavigationSystemV1|GetRandomLocationinNavigableRadius (Transformation|GetActorLocation (Game|Player|GetPlayerPawn 0)) 3e+03 0 0))
    (if _returnvalue
      (switch int (Math|Random|RandomIntegerinRange 0 2)
        (:0
          (Game|SpawnActorfromClass "/Game/ai/BP_ChildEnemy1.BP_ChildEnemy1_C" (Math|Transform|MakeTransform _randomlocation) "Undefined" 0 0))
        (:1
          (Game|SpawnActorfromClass "/Game/ai/BP_ChildEnemy2.BP_ChildEnemy2_C" (Math|Transform|MakeTransform _randomlocation) "Undefined" 0 0))
        (:2
          (Game|SpawnActorfromClass "/Game/ai/BP_ChildEnemy3.BP_ChildEnemy3_C" (Math|Transform|MakeTransform _randomlocation) "Undefined" 0 0)))
      (Variables|Default|SetEnemyCounter (+ (Variables|Default|GetEnemyCounter) 1)))
    (else
      (Utilities|Time|ClearandInvalidateTimerbyHandle (Variables|Default|GetSpawnTimter)))))

(event EventBeginPlay
  (bind _returnvalue (Utilities|Time|SetTimerbyEvent (delegate Custom|SpawnEnemy) (Variables|Default|GetSpawnTime) true))
  (Variables|Default|SetSpawnTimter _returnvalue))

(fn ConstructionScript)