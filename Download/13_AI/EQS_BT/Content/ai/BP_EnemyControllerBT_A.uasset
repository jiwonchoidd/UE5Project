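; Enemy AI controller that runs the BT_Enemy1 behavior tree on possession and feeds player perception into its blackboard.
; Sensing an actor tagged Player cancels the pending timer, sets HasLineOfSight and stores the actor as EnemyActor.
; Any other perception update starts a short one-shot timer that clears both keys, so the enemy keeps its target briefly after losing the player.
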(event OnTargetPerceptionUpdated(AIPerception)
  (params (Actor :type Actor%20Object%20Reference) (Stimulus :type AI%20Stimulus%20Structure))
  (bind _returnvalue (AI|GetBlackboard 0))
  ;[1 1 1] 코멘트
  (if (and (Actor|ActorHasTag Actor "Player") (.bSuccessfullySensed (Utilities|Struct|BreakAIStimulus Stimulus)))
    (Utilities|Time|ClearandInvalidateTimerbyHandle (Variables|Default|GetHandle))
    (AI|Components|Blackboard|SetValueasBool _returnvalue (Variables|Default|GetHasLIneOfSight) true)
    (AI|Components|Blackboard|SetValueasObject _returnvalue (Variables|Default|GetEnemyActor) Actor)
    (else
      (bind _returnvalue_2 (Utilities|Time|SetTimerbyEvent (delegate Custom|StartEnemyTimer) 3.0))
      (Variables|Default|SetHandle _returnvalue_2))))

(event Custom|StartEnemyTimer
  (bind _returnvalue (AI|GetBlackboard 0))
  ;[1 1 1] 코멘트
  (AI|Components|Blackboard|SetValueasBool _returnvalue (Variables|Default|GetHasLineOfSight) false)
  (AI|Components|Blackboard|SetValueasObject _returnvalue (Variables|Default|GetEnemyActor) 0))

(event EventPossess
  (params (PossessedPawn :type Pawn%20Object%20Reference))
  ;[1 1 1] 코멘트
  (AI|RunBehaviorTree "/Game/ai/BT_Enemy1.BT_Enemy1"))

(fn ConstructionScript)