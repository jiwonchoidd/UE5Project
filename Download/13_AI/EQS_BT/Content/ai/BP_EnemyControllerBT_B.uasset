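; Enemy AI controller that runs the BT_EnemyEQS1 behavior tree on possession and feeds it perception results through the blackboard.
; Sensing an actor tagged Player cancels the lost-sight timer, sets HasLineOfSight and stores that actor as TargetActor.
; Any other perception update clears HasLineOfSight immediately and starts an eight-second timer that empties TargetActor, so the target outlasts brief losses of sight.
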(event OnTargetPerceptionUpdated(AIPerception)
  (params (Actor :type Actor%20Object%20Reference) (Stimulus :type AI%20Stimulus%20Structure))
  ;[1 1 1] 코멘트
  (Variables|Default|SetPerceivedActor Actor)
  (if (and (Actor|ActorHasTag Actor "Player") (.bSuccessfullySensed (Utilities|Struct|BreakAIStimulus Stimulus)))
    (Utilities|Time|ClearandInvalidateTimerbyHandle (Variables|Default|GetLostSightTimer))
    (CallFunction|UpdateSightKey true)
    (CallFunction|UpdateTargetKey (Variables|Default|GetPerceivedActor))
    (else
      (bind _returnvalue (Utilities|Time|SetTimerbyEvent (delegate Custom|LostSigt) 8.0))
      (Variables|Default|SetLostSightTimer _returnvalue)
      (CallFunction|UpdateSightKey false))))

(event Custom|LostSigt
  ;[1 1 1] 코멘트
  (CallFunction|UpdateTargetKey))

(event EventBeginPlay)

(event EventTick
  (params (DeltaSeconds :type Float%20%28single-precision%29)))

(event EventPossess
  (params (PossessedPawn :type Pawn%20Object%20Reference))
  (AI|RunBehaviorTree "/Game/ai/BT_EnemyEQS1.BT_EnemyEQS1"))

(fn ConstructionScript)

(fn UpdateSightKey
  (params (HasLineSight :type Boolean))
  (AI|Components|Blackboard|SetValueasBool (Variables|Default|GetBlackboard) (Utilities|Name|MakeLiteralName "HasLineOfSight") HasLineSight))

(fn UpdateTargetKey
  (params (TargetActor :type Actor%20Object%20Reference))
  (AI|Components|Blackboard|SetValueasObject (Variables|Default|GetBlackboard) (Utilities|Name|MakeLiteralName "TargetActor") TargetActor))