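; EnemyPatrol is an AI enemy that patrols waypoints and chases actors it perceives.
; From a random starting Waypoint, move-completed events advance it along NextWaypoint links with randomized pauses.
; AI Perception updates drive an integer state from patrol through detection to chase, focusing and moving to a target in line of sight.
; When TimeoutChase is set, Tick uses line-of-sight checks and a retriggerable delay to abandon the chase and resume patrol.
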(event OnPerceptionUpdated(AIPerception)
  (params (UpdatedActors :type Array%20of%20Actor%20Object%20References))
  ;[1 1 1] 자신이 아닌 감지된 EnemyActor가 있다면 상태 전환한다.
  (CallFunction|DetectedEnemies UpdatedActors))

(event Custom|NextRoute
  (bind _currentpoint (Variables|Step1|GetCurrentPoint))
  ;[1 1 1] CurrentPoint로 이동한다.
  (if (== (Variables|Step1|GetState) 0)
    (Utilities|GetAiController
      (:Found
        (Utilities|IsValid _currentpoint
          (:Is%20Valid
            (AI|Navigation|MovetoActor _currentpoint -1.0 true true true 0)))))))

(event Custom|ReceiveMoveCompleted_Event_0
  (params (RequestID :type AI%20Request%20ID%20Structure) (Result :type EPathFollowingResult%20Enum :default "Success"))
  ;[1 1 1] 모든 웨이포인트를 검색하고 연결리스트화 된 웨이포인트를 사용하여 다음 장소를 얻는다.
  (switch Utilities|FlowControl|Switch|SwitchonEPathFollowingResult Result
    (:Success
      (if (== (Variables|Step1|GetState) 0)
        (Utilities|FlowControl|RetriggerableDelay 0.2)
        (Utilities|IsValid (Variables|Step1|GetCurrentPoint)
          (:Is%20Valid
            (Variables|Step1|SetCurrentPoint (Variables|/Game/Blueprint/Waypoint.Waypoint_C|GetNextWaypoint (Variables|Step1|GetCurrentPoint)))
            (Utilities|FlowControl|Delay (+ (Math|Random|RandomFloatinRange 0.0 (Variables|Step1|GetRoutePauseDeviation)) (Variables|Step1|GetRoutePauseDelay)))
            (CallFunction|NextRoute)))))))

(event Custom|Detected%20Enemies
  (params (Detected%20Actors :type Array%20of%20Actor%20Object%20References))
  ;[1 1 1] 자신이 아닌 감지된 EnemyActor가 있다면 상태 전환한다.
  (if (== (Variables|Step1|GetState) 0)
    (if (>= (Utilities|Array|Length Detected%20Actors) 1)
      (Variables|Step1|SetState 1)
      (switch int (Variables|Step1|GetState) :!label _label
        (:1
          ;[1 1 1] 시야에 들어온 새로운 Enemy Actor이 있다면 공격상태(2)로 전환 및 이동한다.
          (bind _returnvalue (Utilities|GetAiController)
            (:Found
              (bind _array_element (Utilities|Array|ForEachLoopwithBreak Detected%20Actors :!label _label_2)
                (:LoopBody
                  (if (Controller|LineOfSightTo _array_element "0, 0, 0" false)
                    (if (not (Utilities|IsValid (Variables|Default|GetEnemyActor)))
                      (bind _output_get (Variables|Default|SetEnemyActor _array_element))
                      (AI|SetFocus _returnvalue)
                      (bind _returnvalue_2 (AI|Navigation|MovetoActor _returnvalue _output_get -1.0 true true true 0))
                      (switch Utilities|FlowControl|Switch|SwitchonEPathFollowingRequestResult _returnvalue_2
                        (:RequestSuccessful
                          (Variables|Step1|SetState 2)
                          (goto _label_2 Break))))
                    (else
                      ;[1 1 1] 시야에서 Enmemy Actor이 사라지면 NULL 및 걷기 상태로 전환한다.
                      (if (== _array_element (Variables|Default|GetEnemyActor))
                        (Variables|Default|SetEnemyActor 0)
                        (AI|SetFocus)
                        (Variables|Step1|SetState 0)))))))))
        (:2
          ;[1 1 1] 감지된 유저로 이동한다. 상태=2일 경우
          (bind _returnvalue_3 (Utilities|GetAiController)
            (:Found
              (Utilities|IsValid (Variables|Default|GetEnemyActor)
                (:Is%20Valid
                  (AI|Navigation|MovetoActor _returnvalue_3 (Variables|Default|GetEnemyActor) -1.0 true true true 0))))))))
    (else
      (goto _label))))

(event EventBeginPlay
  ;[1 1 1] 모든 웨이포인트를 검색하고 연결리스트화 된 웨이포인트를 사용하여 다음 장소를 얻는다.
  (bind _returnvalue (Utilities|GetAiController)
    (:Found
      (bind _outactors (Actor|GetAllActorsOfClass "/Game/Blueprint/Waypoint.Waypoint_C"))
      (Variables|Step1|SetCurrentPoint (Utilities|Array|Get(acopy) _outactors (Math|Random|RandomInteger (- (Utilities|Array|Length _outactors) 1))))
      (EventDispatchers|BindEventtoReceiveMoveCompleted _returnvalue (delegate Custom|ReceiveMoveCompleted_Event_0))
      (CallFunction|NextRoute))))

(event EventTick
  (params (DeltaSeconds :type Float%20%28single-precision%29))
  ;[1 1 1] Step #3
  (if (== (Variables|Step1|GetState) 2)
    (bind _returnvalue (Utilities|GetAiController)
      (:Found
        (if (Variables|디폴트|GetTimeoutChase)
          (if (Controller|LineOfSightTo (Variables|Default|GetEnemyActor) "0, 0, 0" false)
            (Utilities|FlowControl|Sequence
              (:then_0
                (Utilities|FlowControl|RetriggerableDelay (Variables|디폴트|GetChaseTime))
                (goto _label Reset)))
            (else
              (Utilities|FlowControl|DoOnce false :!label _label
                (:Completed
                  (AI|Navigation|StopMovement _returnvalue)
                  (Variables|Default|SetEnemyActor 0)
                  (Variables|Step1|SetState 0)
                  (CallFunction|NextRoute))))))))))

(fn ConstructionScript)