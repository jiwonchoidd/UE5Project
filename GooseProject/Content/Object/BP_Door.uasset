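; BP_Door is a swinging door actor that opens in response to a player overlap event and closes itself.
; On BeginPlay it binds DoorEvent to the player-overlapped event of BP_ThirdPersonCharacter actors, rather than using its own overlap event.
; DoorEvent plays a timeline that lerps the door's relative yaw open.
; When the timeline finishes, a retriggerable delay leads to CloseDoor, which reverses it if IsOpen is set.
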(event Custom|DoorEvent
  (bind _opentime (Timeline|TimeLine Play)
    (:Update
      (Transformation|SetRelativeRotation (Variables|Default|GetDoor) (Math|Rotator|MakeRotator 0.0 0.0 (Math|Float|Lerp 0.0 1.2e+02 _opentime)) false false)
      (Variables|Default|SetisOpen true))
    (:Finished
      (Utilities|FlowControl|RetriggerableDelay 4.0)
      (CallFunction|CloseDoor)
      (Variables|Default|SetisOpen false))))

(event Custom|CloseDoor
  (if (not (not (Variables|Default|GetisOpen)))
    (bind _opentime (Timeline|TimeLine Reverse)
      (:Update
        (Transformation|SetRelativeRotation (Variables|Default|GetDoor) (Math|Rotator|MakeRotator 0.0 0.0 (Math|Float|Lerp 0.0 1.2e+02 _opentime)) false false)
        (Variables|Default|SetisOpen true))
      (:Finished
        (Utilities|FlowControl|RetriggerableDelay 4.0)
        (CallFunction|CloseDoor)
        (Variables|Default|SetisOpen false)))))

(event EventBeginPlay
  (bind _outactors (Actor|GetAllActorsOfClass "/Game/ThirdPersonBP/BluePrint/BP_ThirdPersonCharacter.BP_ThirdPersonCharacter_C"))
  (EventDispatchers|BindEventtoPlayerOverlapped _outactors (delegate Custom|DoorEvent)))

(event Collision|EventActorBeginOverlap
  (params (OtherActor :type Actor%20Object%20Reference)))

(event EventTick
  (params (DeltaSeconds :type Float%20%28single-precision%29)))

(fn ConstructionScript)