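; BP_Sphere is an actor that toggles its point light and briefly simulates physics in response to overlap notifications from the player character.
; On BeginPlay it finds BP_ThirdPersonCharacter actors and binds its Overlapped event to their PlayerOverlapped dispatcher.
; A FlipFlop alternates each notification between lighting up with one second of sphere physics and switching the light off.
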(event Custom|Overlapped
  ;[1 1 1] 라이트
  (Utilities|FlowControl|FlipFlop
    (:A
      (Rendering|SetVisibility (Variables|Default|GetPointLight) true false)
      (Physics|SetSimulatePhysics (Variables|Default|GetSphere) true)
      (Utilities|FlowControl|Delay 1.0)
      (Physics|SetSimulatePhysics (Variables|Default|GetSphere) false))
    (:B
      (Rendering|SetVisibility (Variables|Default|GetPointLight) false false))))

(event Collision|EventActorBeginOverlap
  (params (OtherActor :type Actor%20Object%20Reference)))

(event EventTick
  (params (DeltaSeconds :type Float%20%28single-precision%29)))

(event EventBeginPlay
  (bind _outactors (Actor|GetAllActorsOfClass "/Game/ThirdPersonBP/BluePrint/BP_ThirdPersonCharacter.BP_ThirdPersonCharacter_C"))
  (EventDispatchers|BindEventtoPlayerOverlapped _outactors (delegate Custom|Overlapped)))

(fn ConstructionScript)