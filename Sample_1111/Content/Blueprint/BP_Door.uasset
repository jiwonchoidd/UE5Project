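; A door actor that swings open and closes itself again, triggered by a table's event dispatcher or its own Interact event.
; On BeginPlay it binds DoorEvent to the dispatcher of the first BP_Table found in the level.
; A timeline lerps the door mesh's yaw to swing it open.
; When the timeline finishes, a retriggerable delay leads to CloseDoor, which reverses it.
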(event Custom|DoorEvent
  (bind _time (Timeline|TimeLineDoor Play)
    (:Update
      (Transformation|SetRelativeRotation (Variables|Default|GetSM_Door) (Math|Rotator|MakeRotator 0.0 0.0 (Math|Float|Lerp 0.0 1.2e+02 _time)) false false))
    (:Finished
      (Utilities|FlowControl|RetriggerableDelay 4.0)
      (CallFunction|CloseDoor))))

(event Custom|CloseDoor
  (bind _time (Timeline|TimeLineDoor Reverse)
    (:Update
      (Transformation|SetRelativeRotation (Variables|Default|GetSM_Door) (Math|Rotator|MakeRotator 0.0 0.0 (Math|Float|Lerp 0.0 1.2e+02 _time)) false false))
    (:Finished
      (Utilities|FlowControl|RetriggerableDelay 4.0)
      (CallFunction|CloseDoor))))

(event EventBeginPlay
  (bind _outactors (Actor|GetAllActorsOfClass "/Game/Blueprint/BP_Table.BP_Table_C"))
  (EventDispatchers|BindEventtoEDEventDispather (Utilities|Array|Get(acopy) _outactors) (delegate Custom|DoorEvent)))

(event Collision|EventActorBeginOverlap
  (params (OtherActor :type Actor%20Object%20Reference)))

(event EventTick
  (params (DeltaSeconds :type Float%20%28single-precision%29)))

(event EventInteract
  (bind _time (Timeline|TimeLineDoor Play)
    (:Update
      (Transformation|SetRelativeRotation (Variables|Default|GetSM_Door) (Math|Rotator|MakeRotator 0.0 0.0 (Math|Float|Lerp 0.0 1.2e+02 _time)) false false))
    (:Finished
      (Utilities|FlowControl|RetriggerableDelay 4.0)
      (CallFunction|CloseDoor))))

(fn ConstructionScript)