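; BP_Table is an actor that signals lamps in the level, apparently as an exercise in event dispatchers.
; On BeginPlay it gathers every BP_Lamp into an array and calls EventLamp on each.
; Overlapping its Sphere component broadcasts the EDEventDispather dispatcher, whose listeners are not shown here.
; Unconnected leftover nodes for spawning an actor, toggling a light and binding to the dispatcher never run.
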(event OnComponentBeginOverlap(Sphere)
  (params (OverlappedComponent :type Primitive%20Component%20Object%20Reference) (OtherActor :type Actor%20Object%20Reference) (OtherComp :type Primitive%20Component%20Object%20Reference) (OtherBodyIndex :type Integer) (bFromSweep :type Boolean) (SweepResult :type Hit%20Result%20Structure%20%28by%20ref%29))
  ;[1 1 1] 디스패처 호출
  (Default|CallEDEventDispather) ; 이벤트 디스패처
)

(event EventBeginPlay
  ;[1 1 1] 디스패처 호출
  (bind _outactors (Actor|GetAllActorsOfClass "/Game/Blueprint/BP_Lamp.BP_Lamp_C"))
  (bind _output_get (Variables|Default|Setlamparray _outactors))
  (for _array_element _output_get
    (Default|EventLamp _array_element)))

(event Collision|EventActorBeginOverlap
  (params (OtherActor :type Actor%20Object%20Reference)))

(event EventTick
  (params (DeltaSeconds :type Float%20%28single-precision%29)))

(fn ConstructionScript)