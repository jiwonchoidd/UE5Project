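; Player HUD that draws an aim crosshair texture, shifted from screen centre by the character's camera and weapon orientation.
; BeginPlay caches the first Ue4ASP_Character found in the level.
; Each DrawHUD offsets the crosshair vertically by scaled camera pitch and horizontally by the height difference between the weapon's start and end sockets.
; That weapon offset is recomputed after drawing, so it applies one frame later.
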(event EventBeginPlay
  (bind _outactors (Actor|GetAllActorsOfClass "/Game/AnimStarterPack/Ue4ASP_Character.Ue4ASP_Character_C"))
  (bind _asue_4asp_character (Utilities|Casting|CastToUe4ASP_Character (Utilities|Array|Get(acopy) _outactors)))
  (Variables|Default|SetObj_Char _asue_4asp_character))

(event Collision|EventActorBeginOverlap
  (params (OtherActor :type Actor%20Object%20Reference)))

(event EventTick
  (params (DeltaSeconds :type Float%20%28single-precision%29)))

(event EventDrawHUD
  (params (SizeX :type Integer) (SizeY :type Integer))
  (Utilities|FlowControl|Sequence
    (:then_0
      (Class|HUD|DrawTextureSimple "/Game/Images/Aim.Aim" (+ (/ SizeX 2) (stale _returnvalue_x)) (+ (/ SizeY 2) (* (.pitch (Transformation|GetWorldRotation (Variables|/Game/AnimStarterPack/Ue4ASP_Character.Ue4ASP_Character_C|GetPlayerCamera (Variables|Default|GetObj_Char)))) 1e+01)) 0.03 false))
    (:then_1
      (bind _returnvalue_x (CallFunction|WeaponLocation)))))

(fn ConstructionScript)

(fn WeaponLocation
  (bind _obj_char (Variables|Default|GetObj_Char))
  (bind _weapon (Variables|/Game/AnimStarterPack/Ue4ASP_Character.Ue4ASP_Character_C|GetWeapon _obj_char))
  (return (.z (- (Transformation|GetSocketLocation _weapon "Socket_End") (Transformation|GetSocketLocation _weapon "Socket_Start")))))