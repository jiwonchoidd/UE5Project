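; BP_PlayerHud is a HUD Blueprint that draws a small aim crosshair texture on screen.
; On BeginPlay it caches the first BP_Mixamo1 actor found in the level as the player character.
; Each DrawHUD offsets the crosshair from screen center, vertically by the scaled player camera pitch and horizontally by a weapon location value.
; That horizontal value refreshes after drawing from WeaponLocation, which currently always returns zero.
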(event EventBeginPlay
  (bind _outactors (Actor|GetAllActorsOfClass "/Game/Models/BP_Mixamo1.BP_Mixamo1_C"))
  (bind _asbp_mixamo_1 (Utilities|Casting|CastToBP_Mixamo1 (Utilities|Array|Get(acopy) _outactors)))
  (Variables|Default|SetObj_Char _asbp_mixamo_1))

(event Collision|EventActorBeginOverlap
  (params (OtherActor :type Actor%20Object%20Reference)))

(event EventTick
  (params (DeltaSeconds :type Float%20%28single-precision%29)))

(event EventDrawHUD
  (params (SizeX :type Integer) (SizeY :type Integer))
  (Utilities|FlowControl|Sequence
    (:then_0
      (Class|HUD|DrawTextureSimple "/Game/Images/Aim.Aim" (+ (/ SizeX 2) (stale _returnvalue_x)) (+ (/ SizeY 2) (* (.pitch (Transformation|GetWorldRotation (Variables|/Game/Models/BP_Mixamo1.BP_Mixamo1_C|GetPlayerCamera (Variables|Default|GetObj_Char)))) 1e+01)) 0.03 false))
    (:then_1
      (bind _returnvalue_x (CallFunction|WeaponLocation)))))

(fn ConstructionScript)

(fn WeaponLocation
  (return 0.0))